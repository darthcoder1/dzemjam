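; Base door actor that slides its static mesh vertically when an interaction starts.
; The interaction event captures the mesh's current world location, then plays the AnimateDoor timeline, which offsets Z by progress times HeighOffset without sweeping.
; It immediately stops the interaction on InteractableComponentBP while the timeline runs.
; No closing logic exists here, and StopAnimation is an empty event.
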(event Custom|StopAnimation)

(event EventBeginPlay
  (|CallParentFunction) ; This node is disabled and will not be called.\nDrag off pins to build functionality.
)

(event Collision|EventActorBeginOverlap
  (params (OtherActor :type Actor%20Object%20Reference))
  (|CallParentFunction OtherActor) ; This node is disabled and will not be called.\nDrag off pins to build functionality.
)

(event EventTick
  (params (DeltaSeconds :type Float%20%28single-precision%29))
  (|CallParentFunction DeltaSeconds) ; This node is disabled and will not be called.\nDrag off pins to build functionality.
)

(event EventOnInteractionStatedEvent
  (params (InteractingComp :type Interaction%20Component%20BP%20Object%20Reference))
  (Variables|Default|SetStartLocation (Transformation|GetWorldLocation (Variables|Default|GetStaticMesh)))
  (Utilities|FlowControl|Sequence
    (:then_0
      (bind _animprogress (Timeline|AnimateDoor Play)
        (:Update
          (Transformation|SetWorldLocation (Variables|Default|GetStaticMesh) (+ (Variables|Default|GetStartLocation) (Math|Vector|MakeVector 0.0 0.0 (* _animprogress (Variables|Default|GetHeighOffset)))) false false))))
    (:then_1
      (Default|StopInteraction (Variables|Default|GetInteractableComponent_BP) InteractingComp))))

(fn ConstructionScript
  (|CallParentFunction))