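; Hackable security camera that sweeps its yaw on a server-run timeline after a start delay and raises the threat meter while it sees a pawn.
; Each tick, a sphere overlap plus forward-vector angle test detects pawns without an occlusion trace, coloring a debug cone.
; Successful interaction disables detection and stops rotation, while failure re-enables the interactable after a delay.
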(event EventBeginPlay
  (|CallParentFunction)
  (if (Networking|IsServer)
    (Variables|Default|SetStartRotation (.rotation (Transformation|GetActorTransform)))
    (Utilities|FlowControl|Delay (Variables|Default|GetStartDelay))
    (if (Variables|Default|GetreverseRotation)
      (bind _rot (Timeline|Rotate Play)
        (:Update
          (Transformation|SetActorRotation (Math|Rotator|MakeRotator (.roll (Variables|Default|GetStartRotation)) (.pitch (Variables|Default|GetStartRotation)) (+ (.yaw (Variables|Default|GetStartRotation)) (* _rot (Variables|Default|GetMaxRotationAmount)))))))
      (else
        (Timeline|Rotate Reverse)))))

(event EventOnInteractionFinishedEvent
  (params (isSuccess :type Boolean))
  (bind _startrotation (Variables|Default|GetStartRotation))
  (if isSuccess
    (Variables|Default|SetisCameraEnabled false)
    (bind _rot (Timeline|Rotate Stop)
      (:Update
        (Transformation|SetActorRotation (Math|Rotator|MakeRotator (.roll _startrotation) (.pitch _startrotation) (+ (.yaw _startrotation) (* _rot (Variables|Default|GetMaxRotationAmount)))))))
    (else
      (Utilities|FlowControl|Delay 5.0)
      (Variables|/Game/Blueprints/Components/InteractableComponent_BP.InteractableComponent_BP_C|SetisEnabled (Variables|Default|GetInteractableComponent_BP) true))))

(event EventTick
  (params (DeltaSeconds :type Float%20%28single-precision%29))
  (bind _self self)
  (if (Variables|Default|GetisCameraEnabled)
    (Variables|Default|SettargetInSight false)
    (bind (_outactors _returnvalue) (Collision|SphereOverlapActors (Transformation|GetActorLocation) (Variables|Default|GetRadius) (Utilities|Array|MakeArray "ObjectTypeQuery3") 0))
    (if _returnvalue
      (for _array_element _outactors
        (if (<= (Class|KismetMathLibrary|DegAcos (Math|Vector|DotProduct (Math|Vector|GetForwardVector (Transformation|GetActorRotation _self)) (Math|Vector|GetUnitDirection(Vector) (Transformation|GetActorLocation _self) (Transformation|GetActorLocation _array_element)))) (Variables|Default|GetMaxAngle))
          (Variables|Default|SettargetInSight true))))
    (CallFunction|DrawDebugCone (Variables|Default|GettargetInSight))
    (if (Variables|Default|GettargetInSight)
      (if (Networking|IsServer)
        (Class|ThreatMeter|IncreaseThreat (Variables|Default|GetThreatMeter) 0.001)))))

(event EventOnInteractionStatedEvent
  (params (InteractingComp :type Interaction%20Component%20BP%20Object%20Reference)))

(fn ConstructionScript
  (|CallParentFunction))

(fn DrawDebugCone
  (params (targetInSight :type Boolean))
  (if targetInSight
    (LocalVariables|SetCurrentColor (Variables|Default|GetInSightConeColor))
    (else
      (LocalVariables|SetCurrentColor (Variables|Default|GetNotInSightConeColor))))
  (Class|KismetSystemLibrary|DrawDebugConeinDegrees (Transformation|GetActorLocation) (Math|Rotator|GetRotationXVector (Transformation|GetActorRotation)) (Variables|Default|GetRadius) (Variables|Default|GetMaxAngle) 3e+01 12 (LocalVariables|GetCurrentColor) 0.0 3.0))