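; SpeedyLaserTrap_BP is a laser trap actor that raises the threat meter when triggered and can be removed by interacting with it.
; An overlap on its damage collision, handled only on the server, prints a debug "DAMAGE" message and increases threat by a small fixed amount, without applying actual damage.
; Starting an interaction immediately stops it and destroys the collision and mesh components, leaving the actor itself in place.
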(event OnComponentBeginOverlap(DamageCollision)
  (params (OverlappedComponent :type Primitive%20Component%20Object%20Reference) (OtherActor :type Actor%20Object%20Reference) (OtherComp :type Primitive%20Component%20Object%20Reference) (OtherBodyIndex :type Integer) (bFromSweep :type Boolean) (SweepResult :type Hit%20Result%20Structure%20%28by%20ref%29))
  (if (Networking|IsServer)
    (Development|PrintString "DAMAGE")
    (Class|ThreatMeter|IncreaseThreat (Variables|Default|GetThreatMeter) 0.05)))

(event Custom|DestroyComps
  (Components|DestroyComponent (Variables|Default|GetDamageCollision)))

(event EventBeginPlay
  (|CallParentFunction) ; This node is disabled and will not be called.\nDrag off pins to build functionality.
)

(event Collision|EventActorBeginOverlap
  (params (OtherActor :type Actor%20Object%20Reference))
  (|CallParentFunction OtherActor) ; This node is disabled and will not be called.\nDrag off pins to build functionality.
)

(event EventTick
  (params (DeltaSeconds :type Float%20%28single-precision%29))
  (|CallParentFunction DeltaSeconds) ; This node is disabled and will not be called.\nDrag off pins to build functionality.
)

(event EventOnInteractionStatedEvent
  (params (InteractingComp :type Interaction%20Component%20BP%20Object%20Reference))
  (Default|StopInteraction (Variables|Default|GetInteractableComponent_BP) InteractingComp)
  (CallFunction|DestroyComps))

(fn ConstructionScript
  (|CallParentFunction))