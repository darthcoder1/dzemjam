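; AlarmRaisingActor_BP is an interactable actor that raises the threat level when an interaction with it starts.
; Its interaction event adds a small fixed increase to ThreatMeter, then immediately stops the interaction on InteractableComponentBP for the interacting component, so each use acts as a one-shot trigger.
; BeginPlay, overlap and Tick are disabled stubs, and the construction script only calls its parent.
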(event EventBeginPlay
  (|CallParentFunction) ; This node is disabled and will not be called.\nDrag off pins to build functionality.
)

(event Collision|EventActorBeginOverlap
  (params (OtherActor :type Actor%20Object%20Reference))
  (|CallParentFunction OtherActor) ; This node is disabled and will not be called.\nDrag off pins to build functionality.
)

(event EventTick
  (params (DeltaSeconds :type Float%20%28single-precision%29))
  (|CallParentFunction DeltaSeconds) ; This node is disabled and will not be called.\nDrag off pins to build functionality.
)

(event EventOnInteractionStatedEvent
  (params (InteractingComp :type Interaction%20Component%20BP%20Object%20Reference))
  (Class|ThreatMeter|IncreaseThreat (Variables|Default|GetThreatMeter) 0.05)
  (Default|StopInteraction (Variables|Default|GetInteractableComponent_BP) InteractingComp))

(fn ConstructionScript
  (|CallParentFunction))