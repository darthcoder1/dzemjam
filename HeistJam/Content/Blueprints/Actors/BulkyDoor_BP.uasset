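; BulkyDoor_BP is a heavy door actor that lifts and struggles while an interaction is in progress.
; When interaction starts, it caches the mesh's world location, then chains a half-lift timeline into a struggle timeline, both driving vertical position scaled by HeighOffset.
; Finishing the interaction stops only the struggle timeline, and a failed attempt also increases the ThreatMeter.
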(event EventBeginPlay
  (|CallParentFunction))

(event Collision|EventActorBeginOverlap
  (params (OtherActor :type Actor%20Object%20Reference))
  (|CallParentFunction OtherActor) ; This node is disabled and will not be called.\nDrag off pins to build functionality.
)

(event EventTick
  (params (DeltaSeconds :type Float%20%28single-precision%29))
  (|CallParentFunction DeltaSeconds) ; This node is disabled and will not be called.\nDrag off pins to build functionality.
)

(event EventOnInteractionFinishedEvent
  (params (isSuccess :type Boolean))
  (if isSuccess
    (bind _animprogress (Timeline|Timeline_Struggle Stop)
      (:Update
        (Transformation|SetWorldLocation (Variables|Default|GetStaticMesh) (+ (Variables|Default|GetStartLocation) (Math|Vector|MakeVector 0.0 0.0 (* _animprogress (Variables|Default|GetHeighOffset)))) false false)))
    (else
      (Class|ThreatMeter|IncreaseThreat (Variables|Default|GetThreatMeter) 0.1)
      (Timeline|Timeline_Struggle Stop))))

(event EventOnInteractionStatedEvent
  (params (InteractingComp :type Interaction%20Component%20BP%20Object%20Reference))
  (Variables|Default|SetStartLocation (Transformation|GetWorldLocation (Variables|Default|GetStaticMesh)))
  (Utilities|FlowControl|Sequence
    (:then_0
      (bind _animprogress (Timeline|Timeline_HalfLift Play)
        (:Update
          (Transformation|SetWorldLocation (Variables|Default|GetStaticMesh) (+ (Variables|Default|GetStartLocation) (Math|Vector|MakeVector 0.0 0.0 (* _animprogress (Variables|Default|GetHeighOffset)))) false false))
        (:Finished
          (bind _animprogress_2 (Timeline|Timeline_Struggle Play)
            (:Update
              (Transformation|SetWorldLocation (Variables|Default|GetStaticMesh) (+ (Variables|Default|GetStartLocation) (Math|Vector|MakeVector 0.0 0.0 (* _animprogress_2 (Variables|Default|GetHeighOffset)))) false false))))))))

(fn ConstructionScript
  (|CallParentFunction))