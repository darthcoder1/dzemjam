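; InteractableComponent_BP is a component that makes its owning actor interactable and tracks whether it is enabled or in use.
; StartInteraction marks it in use, stores the interacting component and calls InteractionStarted.
; StopInteraction disables it and notifies the interacting component through ClientOnInteractionFinished.
; RepNotifies on both flags drive the Interaction_WBP in the owner's WidgetComponent, showing availability while in use and collapsing it once disabled.
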(event Custom|StartInteraction
  (params (InteractingComponent :type Interaction%20Component%20BP%20Object%20Reference))
  (Variables|Default|SetisBeingUsed true)
  (bind _output_get (Variables|Default|SetCurrentInteractingComponent InteractingComponent))
  (Default|CallInteractionStarted _output_get))

(event Custom|StopInteraction
  (params (InteractingComp :type Interaction%20Component%20BP%20Object%20Reference))
  (Variables|Default|SetisEnabled false)
  (Variables|Default|SetisBeingUsed false)
  (Default|ClientonInteractionFinished InteractingComp))

(event EventBeginPlay)

(event EventTick
  (params (DeltaSeconds :type Float%20%28single-precision%29)))

(fn SetInteractionWidgetVisibility
  (params (NewVisibility :type ESlateVisibility%20Enum :default "Visible"))
  (Widget|SetVisibility (CallFunction|GetInteractionWidget) NewVisibility))

(fn SetInteractionWidgetState
  (params (isInteractable :type Boolean))
  (Default|SetInteractionState (CallFunction|GetInteractionWidget) isInteractable))

(fn GetInteractionWidget
  (bind _asinteraction_wbp (Utilities|Casting|CastToInteraction_WBP (UserInterface|GetUserWidgetObject (Actor|GetComponentbyClass (Components|GetOwner) "/Script/UMG.WidgetComponent")))
    (:then
      _)
    (:CastFailed
      _))
  (return _asinteraction_wbp))

(fn OnRepIsBeingUsed
  (CallFunction|SetInteractionWidgetState (not (Variables|Default|GetisBeingUsed))))

(fn OnRepIsEnabled
  (if (not (Variables|Default|GetisEnabled))
    (CallFunction|SetInteractionWidgetVisibility "Collapsed")))