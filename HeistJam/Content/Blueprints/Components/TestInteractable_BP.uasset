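; TestInteractable_BP is a test interactable actor with placeholder logic for exercising the interaction component.
; On BeginPlay it collapses its widget component's user widget, and only the server binds to InteractableComponentBP's interaction-started event.
; When an interaction starts, it waits a fixed delay, then tells the component to stop that interaction for the interacting component.
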(event Custom|InteractionStarted
  (params (InteractingComp :type Interaction%20Component%20BP%20Object%20Reference))
  (Utilities|FlowControl|Delay 4.0) ; slap random login in here...
  (Default|StopInteraction (Variables|Default|GetInteractableComponent_BP) InteractingComp))

(event EventBeginPlay
  (Widget|SetVisibility (UserInterface|GetUserWidgetObject (Variables|Default|GetWidgetComponent)) "Collapsed")
  (if (Networking|IsServer)
    (EventDispatchers|BindEventtoInteractionStarted (Variables|Default|GetInteractableComponent_BP) (delegate Custom|InteractionStarted))))

(event Collision|EventActorBeginOverlap
  (params (OtherActor :type Actor%20Object%20Reference)))

(event EventTick
  (params (DeltaSeconds :type Float%20%28single-precision%29)))

(fn ConstructionScript)