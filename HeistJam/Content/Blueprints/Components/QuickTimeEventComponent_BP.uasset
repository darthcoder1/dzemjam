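; Actor component that runs a chained quick-time event for a player-controlled Character in HeistJam.
; StartQuickTimeEvent binds the controller's four directional press events and opens a Gate, which creates a prompt widget with random key and duration.
; Presses are compared to that key, then the widget's delegate removes it and starts another delayed round until QTEComplexity is reached or an input fails.
; The interaction-stopping OnFinished event is not called by this loop.
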(event Custom|StartQuickTimeEvent
  (CallFunction|OpentheGate)
  (CallFunction|ModularSequences)
  (EventDispatchers|AssignOnQuickTimeEventPressedUp (stale EventBeginPlay _output_get) (delegate Custom|QuickTimeUpPressed))
  (EventDispatchers|BindEventtoOnQuickTimeEventPressedDown (stale EventBeginPlay _output_get) (delegate Custom|QuickTimeDownPressed))
  (EventDispatchers|BindEventtoOnQuickTimeEventPressedRight (stale EventBeginPlay _output_get) (delegate Custom|QuickTimeRightPressed))
  (EventDispatchers|BindEventtoOnQuickTimeEventPressedLeft (stale EventBeginPlay _output_get) (delegate Custom|QuickTimeLeftPressed)))

(event Custom|StartSequence)

(event Custom|modularSequences
  (Math|Integer|IncrementInt (Variables|Default|GetQTELoopCount)
    (:%20%20
      (Utilities|FlowControl|Delay 1.0)
      (Utilities|FlowControl|Gate false
        (:Exit
          (if (Variables|Default|GetrightButtonPressed)
            (bind _output_get (Variables|Default|SetquickTimeInputEnum (Utilities|Enum|ByteToEnumQuickTimeButton (Math|Conversions|ToByte(Integer) (Math|Random|RandomIntegerinRange 1 4)))))
            (bind _returnvalue (UserInterface|CreateWidget "/Game/TopDownCPP/Blueprints/QuickTimeEvent/W_QuickTimeEvent.W_QuickTimeEvent_C" 0 _output_get (Math|Random|RandomFloatinRange 2.0 4.0)))
            (Variables|Default|SetQTEWidget _returnvalue)
            (UserInterface|Viewport|AddtoViewport _returnvalue 0)
            (EventDispatchers|BindEventtoHalloDelegate _returnvalue (delegate Custom|DestroyME))
            (else
              (CallFunction|DestroyME))))))))

(event Custom|DestroyME
  (Widget|RemovefromParent (stale Custom|modularSequences _returnvalue))
  (Variables|Default|SetquickTimeInputEnum "NewEnumerator4")
  (if (and (< (Variables|Default|GetQTELoopCount) (Variables|Default|GetQTEComplexity)) (Variables|Default|GetrightButtonPressed))
    (CallFunction|ModularSequences)
    (else
      (Variables|Default|SetQTELoopCount 0)
      (Variables|Default|SetrightButtonPressed true)
      (CallFunction|ClosetheGate))))

(event Custom|OpenTheGate
  (Utilities|FlowControl|Gate false) ; enters at Open
)

(event Custom|CloseTheGate
  (Utilities|FlowControl|Gate false) ; enters at Close
)

(event Custom|OnFinished
  (params (NewParam :type Boolean))
  (CallFunction|ServerStopInteraction))

(event Custom|ServerStopInteraction
  (Default|StopInteraction (Actor|GetComponentbyClass (Variables|Default|GetClosestActor) "/Game/Blueprints/Components/InteractableComponent_BP.InteractableComponent_BP_C")))

(event Custom|InputPressed
  (params (Key :type QuickTimeButton%20Enum :default "NewEnumerator0"))
  (bind _output_get (Variables|Default|SetrightButtonPressed (Utilities|Enum|Equal(Enum) (Variables|Default|GetquickTimeInputEnum) Key)))
  (Default|CallHalloDelegate (Variables|Default|GetQTEWidget))
  (Development|PrintString (Utilities|String|ToString(Boolean) _output_get)))

(event Custom|QuickTimeUpPressed
  (CallFunction|InputPressed "NewEnumerator0"))

(event Custom|QuickTimeDownPressed
  (CallFunction|InputPressed "NewEnumerator1"))

(event Custom|QuickTimeRightPressed
  (CallFunction|InputPressed "NewEnumerator3"))

(event Custom|QuickTimeLeftPressed
  (CallFunction|InputPressed "NewEnumerator2"))

(event EventBeginPlay
  (bind _ascharacter (Utilities|Casting|CastToCharacter (Components|GetOwner)))
  (bind _asheist_jam_player_controller (Utilities|Casting|CastToHeistJamPlayerController (Pawn|GetController _ascharacter)))
  (bind _output_get (Variables|Default|SetPlayerController _asheist_jam_player_controller)))

(event EventTick
  (params (DeltaSeconds :type Float%20%28single-precision%29)))

(fn NewFunction0
  (params (TimePassed :type Float%20%28single-precision%29)))